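; BP_DrivableCar is a car actor that drives straight along its forward vector while its Started flag is set.
; Each Tick moves it by Speed using a swept teleport offset, with no delta-time scaling, so movement depends on frame rate.
; The four wheel components spin by WheelRotationSpeed on local yaw, negated on the right side.
; The graph contains no input or steering and never sets Started itself.
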(event `self.ReceiveTick`
  (params (DeltaSeconds :type "Float (single-precision)"))
  (bind _wheelrotationspeed (`self.WheelRotationSpeed`))
  (bind _returnvalue (* _wheelrotationspeed -1.0))
  (if (`self.Started`)
    (`self.K2_AddActorWorldOffset` (* (`self.GetActorForwardVector`) (`self.Speed`)) true true)
    (`SceneComponent.K2_AddLocalRotation` (`self.FrontRight`) (`KismetMathLibrary.MakeRotator` 0.0 0.0 _returnvalue) false false)
    (`SceneComponent.K2_AddLocalRotation` (`self.BackRight`) (`KismetMathLibrary.MakeRotator` 0.0 0.0 _returnvalue) false false)
    (`SceneComponent.K2_AddLocalRotation` (`self.FrontLeft`) (`KismetMathLibrary.MakeRotator` 0.0 0.0 _wheelrotationspeed) false false)
    (`SceneComponent.K2_AddLocalRotation` (`self.BackLeft`) (`KismetMathLibrary.MakeRotator` 0.0 0.0 _wheelrotationspeed) false false)))

(fn `UserConstructionScript`)