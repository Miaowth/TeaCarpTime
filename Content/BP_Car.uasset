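; BP_Car is a player-controlled car driven by the MoveForward and MoveRight axes.
; Axis events feed steering and throttle to VehicleMovement, with throttle input also shifting the pitch and volume parameters of CarNoises.
; Separately, Tick yaws the Capsule and moves it along its forward vector with sweep and teleport enabled.
; Tick also spins the four wheel components from forward input, negating the rotation on the left side.
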(event `self.ReceiveBeginPlay`)

(event `InputAxis|MoveRight` :overrideparent false
  (params (AxisValue :type "Float (single-precision)"))
  ;[1 1 1] Steering input
  (`WheeledVehicleMovementComponent.SetSteeringInput` (`self.VehicleMovement`) AxisValue))

(event `InputAxis|MoveForward` :overrideparent false
  (params (AxisValue :type "Float (single-precision)"))
  (bind _carnoises (`self.CarNoises`))
  ;[1 1 1] Throttle input
  (`WheeledVehicleMovementComponent.SetThrottleInput` (`self.VehicleMovement`) AxisValue)
  (`AudioComponent.SetFloatParameter` _carnoises "ModulatorPitch" (+ (`self.PitchModifier`) AxisValue))
  (`AudioComponent.SetFloatParameter` _carnoises "ModulatorVolume" (+ (`self.VolumeModifier`) AxisValue)))

(event `self.ReceiveTick`
  (params (DeltaSeconds :type "Float (single-precision)"))
  (bind _returnvalue (`self.GetInputAxisValue`))
  (bind _capsule (`self.Capsule`))
  (bind _returnvalue_2 (* _returnvalue (`self.WheelSpeed`)))
  (bind _returnvalue_3 (* _returnvalue_2 -1.0))
  (`SceneComponent.K2_AddLocalRotation` (`self.Capsule`) (`KismetMathLibrary.MakeRotator` 0.0 0.0 (`self.GetInputAxisValue`)) false false)
  (`SceneComponent.K2_AddWorldOffset` _capsule (* (* (`SceneComponent.GetForwardVector` _capsule) (`self.Speed`)) _returnvalue) true true)
  (`SceneComponent.K2_AddLocalRotation` (`self.BackRight`) (`KismetMathLibrary.MakeRotator` 0.0 0.0 _returnvalue_2) false false)
  (`SceneComponent.K2_AddLocalRotation` (`self.FrontRight`) (`KismetMathLibrary.MakeRotator` 0.0 0.0 _returnvalue_2) false false)
  (`SceneComponent.K2_AddLocalRotation` (`self.BackLeft`) (`KismetMathLibrary.MakeRotator` 0.0 0.0 _returnvalue_3) false false)
  (`SceneComponent.K2_AddLocalRotation` (`self.FrontLeft`) (`KismetMathLibrary.MakeRotator` 0.0 0.0 _returnvalue_3) false false))

(fn `UserConstructionScript`)